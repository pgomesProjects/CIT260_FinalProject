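; Swinging lamp Blueprint that rocks its Lamp component left and right around the pitch axis.
; Each Tick adds a world rotation of RotationSpeed scaled by DeltaSeconds.
; RotationSpeed steps toward RotationMax by Change, and RotationMax flips sign when reached or overshot, reversing the swing.
; The speed step is per frame, not scaled by DeltaSeconds, so the swing depends on frame rate.
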(event EventTick
  (params (DeltaSeconds :type Float%20%28single-precision%29))
  ;[1 1 1] Swing Lamp Left and Right
  (Utilities|FlowControl|Sequence
    (:then_0
      (Transformation|AddWorldRotation (Variables|Default|GetLamp) (* (Math|Rotator|MakeRotator 0.0 (Variables|Default|GetRotation_Speed) 0.0) DeltaSeconds) false false))
    (:then_1
      (Math|Float|CompareFloat (Variables|Default|GetRotation_Speed) (Variables|Default|GetRotationMax)
        (:>
          (Variables|Default|SetRotation_Speed (- (Variables|Default|GetRotation_Speed) (Variables|Default|GetChange))))
        (:==
          (Variables|Default|SetRotationMax (* (Variables|Default|GetRotationMax) -1.0)))
        (:<
          (Variables|Default|SetRotation_Speed (- (Variables|Default|GetRotation_Speed) (* (Variables|Default|GetChange) -1.0)))
          (Math|Float|CompareFloat (Variables|Default|GetRotation_Speed) (Variables|Default|GetRotationMax)
            (:>
              (Variables|Default|SetRotationMax (* (Variables|Default|GetRotationMax) -1.0)))))))))

(fn ConstructionScript)